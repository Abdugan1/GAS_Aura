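; BP_FadeActor is a static mesh actor that can fade out and back in through a material scalar parameter.
; The construction script caches the original materials and builds dynamic instances from FadeMaterialInstances.
; FadeOut swaps those in and plays a timeline driving their Fade parameter, which Fadein reverses.
; On finish, a value of one restores the originals and blocks the Visibility channel, while zero makes the mesh ignore it.
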(event EventFadeOut
  (CallFunction|UpdateMaterials (Variables|Default|GetDynamic%20Material%20Instances))
  (bind _fade (Timeline|FadeTimeline Play)
    (:Update
      (for _array_element (Variables|Default|GetDynamic%20Material%20Instances)
        (Rendering|Material|SetScalarParameterValue _array_element "Fade" _fade :!class /Script/Engine.MaterialInstanceDynamic)))
    (:Finished
      (CallFunction|FadeFinished _fade))))

(event EventFadein
  (bind _fade (Timeline|FadeTimeline Reverse)
    (:Update
      (for _array_element (Variables|Default|GetDynamic%20Material%20Instances)
        (Rendering|Material|SetScalarParameterValue _array_element "Fade" _fade :!class /Script/Engine.MaterialInstanceDynamic)))
    (:Finished
      (CallFunction|FadeFinished _fade))))

(fn ConstructionScript
  (Utilities|Array|Clear (Variables|Default|GetDynamic%20Material%20Instances))
  (Variables|Default|SetOriginal%20Materials (Rendering|Material|GetMaterials (Variables|Default|GetStaticMesh)))
  (for _array_element (Variables|Default|GetFade%20Material%20Instances)
    (bind _returnvalue (Rendering|Material|CreateDynamicMaterialInstance _array_element "None" "None" :!class /Script/Engine.KismetMaterialLibrary))
    (Utilities|Array|AddUnique (Variables|Default|GetDynamic%20Material%20Instances) _returnvalue)))

(fn UpdateMaterials
  (params (Materials :type Array%20of%20Material%20Interface%20Object%20References))
  (for (_array_element _array_index) Materials
    (Rendering|Material|SetMaterial (Variables|Default|GetStaticMesh) _array_index _array_element)))

(fn FadeFinished
  (params (A :type Float%20%28double-precision%29))
  ;[1 1 1] Reset To Original Materials
  (if (>= A 1.0)
    (CallFunction|UpdateMaterials (Variables|Default|GetOriginal%20Materials))
    (Collision|SetCollisionResponsetoChannel (Variables|Default|GetStaticMesh) "ECC_Visibility" "ECR_Block")
    (if (Variables|Collision|GetBlock%20Visibility)
      (Collision|SetCollisionResponsetoChannel (Variables|Default|GetStaticMesh) "ECC_Visibility" "ECR_Block"))
    (elif (<= A 0.0)
      (Collision|SetCollisionResponsetoChannel (Variables|Default|GetStaticMesh) "ECC_Visibility" "ECR_Ignore")
      (Collision|SetCollisionResponsetoChannel (Variables|Default|GetStaticMesh) "ECC_Visibility" "ECR_Ignore"))))