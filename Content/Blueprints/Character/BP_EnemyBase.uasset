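; Base enemy character Blueprint that supplies cosmetic spawn and death effects plus attack-agnostic facing support.
; On BeginPlay, a timeline drives the mesh's uniform scale.
; Separate mesh and weapon timelines animate the Dissolve parameter on dynamic material instances passed into their events after death.
; SetFacingTarget feeds a location to Motion Warping as the FacingTarget warp target, and Tick only calls the parent.
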(event EventBeginPlay
  (bind _newtrack_0 (Timeline|Timeline Play)
    (:Update
      (Transformation|SetRelativeScale3D (Variables|Character|GetMesh) (Math|Vector|MakeVector _newtrack_0 _newtrack_0 _newtrack_0)))))

(event EventTick
  (params (DeltaSeconds :type Float%20%28single-precision%29))
  (|CallParentFunction DeltaSeconds))

(event EventStartMeshDissolveTimeline
  (params (DynamicMaterialInstance :type Material%20Instance%20Dynamic%20Object%20Reference))
  ;[1 1 1] Dissolve after Death: Mesh
  (bind _dissolvetrack (Timeline|MeshDissolveTimeline Play)
    (:Update
      (Rendering|Material|SetScalarParameterValue DynamicMaterialInstance "Dissolve" _dissolvetrack :!class /Script/Engine.MaterialInstanceDynamic))))

(event EventStartWeaponDissolveTimeline
  (params (DynamicMaterialInstance :type Material%20Instance%20Dynamic%20Object%20Reference))
  ;[1 1 1] Dissolve after Death: Weapon
  (bind _dissolvetrack (Timeline|WeaponDissolveTimeline Play)
    (:Update
      (Rendering|Material|SetScalarParameterValue DynamicMaterialInstance "Dissolve" _dissolvetrack :!class /Script/Engine.MaterialInstanceDynamic))))

(event EventSetFacingTarget
  (params (FacingTarget :type Vector%20%28by%20ref%29 :default "0, 0, 0"))
  (Class|MotionWarpingComponent|AddorUpdateWarpTargetfromLocation (Variables|Default|GetMotionWarping) "FacingTarget" FacingTarget))

(fn ConstructionScript)