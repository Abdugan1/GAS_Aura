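; Arcane Shards gameplay ability that shows a magic circle, waits for a press, then spawns shards around the targeted point.
; The press captures mouse target data, faces the caster toward it and plays the cast montage.
; The montage event spawns a BP_PointCollection and caches its randomly rotated ground points.
; A looping timer fires a Niagara gameplay cue per point, then resets state, destroys the collection and ends the ability.
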(event Custom|SpawnShard
  (if (< (Variables|Default|GetCount) (Variables|Default|GetNum%20Points))
    (bind _output_get (Variables|Default|SetShardSpawnPoint (Transformation|GetWorldLocation (Utilities|Array|Get(acopy) (Variables|Default|GetGroundPoints) (Variables|Default|GetCount)))))
    (Math|Integer|IncrementInt (Variables|Default|GetCount)
      (:%20%20
        ;[0.15 0.15 0.15 0.5] Cue -- the shards spawn here through Niagara
        (Class|GameplayAbility|ExecuteGameplayCuewithParams "(TagName=\"GameplayCue.ArcaneShards\")" (Ability|GameplayCue|MakeGameplayCueParameters :Location (Variables|Default|GetShardSpawnPoint)))))
    (else
      ;[0.15 0.15 0.15 0.5] Since it's executing policy is set per actor, we must reset everything. I COULD RESET EVERYTHING in OnEndAbility, but I'm lazy
      (Variables|Default|SetCount 0)
      (Utilities|Time|ClearandInvalidateTimerbyHandle (Variables|Default|GetShardSpawnTimer))
      ;;[0.15 0.15 0.15 0.5] So it's not activate immediately.
      (Utilities|FlowControl|Delay 0.2)
      (Actor|DestroyActor (Variables|Default|GetPointsCollection))
      (Ability|EndAbility))))

(event Ability|EventActivateAbility
  (Utilities|FlowControl|Sequence
    (:then_0
      (Class|PlayerInterface|ShowMagicCircle(Message) (Ability|GetAvatarActorfromActorInfo) 0))
    (:then_1
      ;[0.15 0.15 0.15 0.5] When the ability is activated, we again wait to press the same button so the player can choose the desired location to spawn shards
      (Ability|Tasks|WaitInputPress false
        (:OnPress
          (bind _datahandle (|TargetDataUnderMouse)
            (:ValidData
              ;[0.15 0.15 0.15 0.5] Montage Thing
              (Class|CombatInterface|SetFacingTarget(Message) (Ability|GetAvatarActorfromActorInfo) (.ImpactPoint (Collision|BreakHitResult (Ability|TargetData|GetHitResultfromTargetData _datahandle))))
              (|PlayMontageandWaitProxy "None" "/Game/Assets/Characters/Aura/Animations/Abilities/AM_Cast_ArcaneShards_Montage.AM_Cast_ArcaneShards_Montage" 1.0 "None" false 1.0 0.0 false
                (:then
                  (Ability|Tasks|WaitGameplayEvent "(TagName=\"Event.Montage.ArcaneShards\")" 0
                    (:then
                      ;[0.15 0.15 0.15 0.5] Hide it immediately after the montage is played
                      (Class|PlayerInterface|HideMagicCircle(Message) (Ability|GetAvatarActorfromActorInfo)))
                    (:EventReceived
                      ;[0.15 0.15 0.15 0.5] We use a custom BP class which has handmade locations to spawn the shards on
                      (bind _returnvalue (Game|SpawnActorfromClass "/Game/Blueprints/AbilitySystem/Aura/Abilities/Arcane/ArcaneShards/BP_PointCollection.BP_PointCollection_C" (Math|Transform|MakeTransform (.ImpactPoint (Collision|BreakHitResult (Ability|TargetData|GetHitResultfromTargetData _datahandle))) "0, 0, 0" "1.000000,1.000000,1.000000") "AlwaysSpawn" "MultiplyWithRoot" 0 0))
                      (Variables|Default|SetPointsCollection _returnvalue)
                      ;[0.15 0.15 0.15 0.5] This is crucial since the function is pure, you might get different results every time as pure functions execute each time they're called
                      (Variables|Default|SetGroundPoints (Class|PointCollection|GetGroundPoints _returnvalue (.ImpactPoint (Collision|BreakHitResult (Ability|TargetData|GetHitResultfromTargetData _datahandle))) (Variables|Default|GetNum%20Points) (Math|Random|RandomFloatinRange 0.0 3.6e+02)))
                      ;[0.15 0.15 0.15 0.5] Async Shards Spawn
                      (bind _returnvalue_2 (Utilities|Time|SetTimerbyEvent (delegate Custom|SpawnShard) (Variables|Default|GetShardSpawnFrequency) true))
                      (Variables|Default|SetShardSpawnTimer _returnvalue_2)
                      ;[0.15 0.15 0.15 0.5] First shard must execute right away
                      (CallFunction|SpawnShard))))))))))))