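; BP_FireBolt is the Fire Bolt ability's projectile actor, with logic to clean up surplus bolts that stop moving.
; Tick compares the current location with the previous frame's and, when the distance moved is at or below MinDistancePerFrame, plays the impact sound, spawns the fire explosion Niagara effect and destroys the actor.
; An author note says this polling stands in for an OnDeath delegate and refers to setting the tick interval low.
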(event EventBeginPlay)

(event Collision|EventActorBeginOverlap
  (params (OtherActor :type Actor%20Object%20Reference)))

(event EventTick
  (params (DeltaSeconds :type Float%20%28single-precision%29))
  ;[0.15 0.15 0.15 0.5] NOTE: Set Tick Interval to a low value! Destroying surplus FireBolts. Actually, I could use OnDeath delegate, but I decided to stick to this approach since I didn't know about it.
  (Variables|Default|SetLocation%20Last%20Frame (Variables|Default|GetLocation%20This%20Frame))
  (Variables|Default|SetLocation%20This%20Frame (Transformation|GetActorLocation))
  (if (<= (Math|Vector|VectorLength (- (Variables|Default|GetLocation%20This%20Frame) (Variables|Default|GetLocation%20Last%20Frame))) (Variables|Default|GetMinDistancePerFrame))
    (Audio|SpawnSoundatLocation "/Game/Assets/Sounds/Abilities/FireBolt/sfx_FireBolt_Impact.sfx_FireBolt_Impact" (Variables|Default|GetLocation%20This%20Frame) "0, 0, 0" 1.0 1.0 0.0 0 0)
    (Niagara|SpawnSystematLocation "/Game/Assets/Effects/Projectiles/FireExplosion/NS_FireExplosion.NS_FireExplosion" (Variables|Default|GetLocation%20This%20Frame))
    (Actor|DestroyActor)))

(fn ConstructionScript)