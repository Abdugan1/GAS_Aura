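; Fire Bolt gameplay ability that casts projectiles toward the location under the mouse.
; After committing, it gets cursor target data, turns the avatar toward the hit point and plays the cast montage.
; The montage's gameplay event triggers SpawnProjectiles with that location and a socket tag.
; Any montage exit ends the ability, printing a debug warning if the event never set its flag.
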(event Ability|EventActivateAbility
  (Ability|CommitAbility)
  (bind _datahandle (|TargetDataUnderMouse)
    (:ValidData
      (bind _output_get (Variables|Default|SetProjectile%20Target%20Location (.Location (Collision|BreakHitResult (Ability|TargetData|GetHitResultfromTargetData _datahandle)))))
      (Class|CombatInterface|SetFacingTarget(Message) (Ability|GetAvatarActorfromActorInfo) _output_get)
      (|PlayMontageandWaitProxy "None" "/Game/Assets/Characters/Aura/Animations/Abilities/AM_CastFireBolt.AM_CastFireBolt" 1.0 "None" false 1.0 0.0 false
        (:then
          (Ability|Tasks|WaitGameplayEvent "(TagName=\"Event.Montage.FireBolt\")" 0
            (:EventReceived
              (Variables|Default|SetNewVar true)
              (Class|AuraFireBolt|SpawnProjectiles (Variables|Default|GetProjectile%20Target%20Location) (Variables|Default|GetProjectile%20Spawn%20Socket%20Tag)))))
        (:OnCompleted
          (if (Variables|Default|GetNewVar) :!label _label
            _
            (else
              (Development|PrintString "Didn't receive anim notify, hence didn't spawn. Do know that I changed Montage Tick Type in AM_CastFireBolt")))
          (Ability|EndAbility))
        (:OnBlendOut
          (goto _label))
        (:OnInterrupted
          (goto _label))
        (:OnCancelled
          (goto _label))))))

(event Ability|EventOnEndAbility
  (params (bWasCancelled :type Boolean)))