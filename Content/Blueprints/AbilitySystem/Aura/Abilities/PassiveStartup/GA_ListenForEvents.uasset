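; Passive gameplay ability that turns gameplay events under the Attributes tag into attribute effects on its owner.
; It keeps listening after activation and, for each event, builds a spec from EventBasedEffectClass and applies it to itself.
; Every tag in AllGameplayTagsSetByCaller gets a SetByCaller magnitude: the event's magnitude on an exact tag match, zero otherwise, so none is left unset.
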(event Ability|EventActivateAbility
  (bind _returnvalue (Ability|GetAbilitySystemComponentfromActorInfo))
  ;[0.15 0.15 0.15 0.5] I think this passive ability is for setting SetByCallerMagnitudes to 0 if they don't have any value. Workaround in Blueprints to not have error messages in the log
  ;[1 1 1] This waits forever since Only Trigger Once is not checked
  (bind _payload (Ability|Tasks|WaitGameplayEvent "(TagName=\"Attributes\")" 0 false false)
    (:EventReceived
      (Variables|Default|SetCurrent%20Event%20Tag (.EventTag (Utilities|Struct|BreakGameplayEventData _payload)))
      (Variables|Default|SetCurrent%20Event%20Magnitude (.EventMagnitude (Utilities|Struct|BreakGameplayEventData _payload)))
      (Variables|Default|SetSpec (GameplayEffects|MakeOutgoingSpec _returnvalue (Variables|Default|GetEventBasedEffectClass) 1.0 (GameplayEffects|MakeEffectContext _returnvalue)))
      (for _array_element (Variables|Default|GetAllGameplayTagsSetByCaller)
        (if (GameplayTags|MatchesTag _array_element (Variables|Default|GetCurrent%20Event%20Tag) true)
          (Ability|GameplayEffect|AssignTagSetbyCallerMagnitude (Variables|Default|GetSpec) (Variables|Default|GetCurrent%20Event%20Tag) (Variables|Default|GetCurrent%20Event%20Magnitude))
          (else
            (Ability|GameplayEffect|AssignTagSetbyCallerMagnitude (Variables|Default|GetSpec) _array_element 0.0))))
      (GameplayEffects|ApplyGameplayEffectSpecToSelf (Ability|GetAbilitySystemComponentfromActorInfo) (Variables|Default|GetSpec)))))

(event Ability|EventOnEndAbility
  (params (bWasCancelled :type Boolean)))