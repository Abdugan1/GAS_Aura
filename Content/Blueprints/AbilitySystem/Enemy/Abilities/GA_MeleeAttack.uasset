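; Enemy melee attack gameplay ability that strikes non-friendly actors near a combat socket.
; On activation it faces the combat target, plays a random tagged attack montage and waits for that montage's gameplay event.
; The event triggers a radius query at the montage's socket, damages each non-friend and fires a melee impact GameplayCue on any hit.
; The ability ends after the event, on montage interruption or cancellation, or without a valid target.
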(event Ability|EventActivateAbility
  (bind _returnvalue (Ability|GetAvatarActorfromActorInfo))
  (bind _returnvalue_2 (Ability|GetAvatarActorfromActorInfo))
  (Variables|Default|SetHasHitTarget false)
  (bind _returnvalue_3 (Class|EnemyInterface|GetCombatTarget(Message) _returnvalue))
  (Utilities|IsValid _returnvalue_3
    (:Is%20Valid
      (Class|CombatInterface|SetFacingTarget(Message) _returnvalue (Transformation|GetActorLocation _returnvalue_3))
      (bind _returnvalue_4 (Class|CombatInterface|GetAttackMontages(Message) _returnvalue))
      ;[1 1 1] It's necessary to store the random value in a local var since it COULD get executed every time a node uses it as it MIGHT be a pure function! Better safe than sorry.
      (bind _output_get (Variables|Default|SetTaggedMontage (Class|AuraDamageGameplayAbility|GetRandomTaggedMontagefromArray _returnvalue_4)))
      (|PlayMontageandWaitProxy "None" (.Montage (Utilities|Struct|BreakTaggedMontage _output_get)) 1.0 "None" true 1.0 0.0 false
        (:then
          (Ability|Tasks|WaitGameplayEvent (.MontageTag (Utilities|Struct|BreakTaggedMontage _output_get)) 0
            (:EventReceived
              (bind _returnvalue_5 (Class|CombatInterface|GetCombatSocketLocation(Message) _returnvalue_2 (.SocketTag (Utilities|Struct|BreakTaggedMontage _output_get))))
              (bind _output_get_2 (Variables|Default|SetCombatSocketLocation _returnvalue_5))
              (bind _outoverlappingactors (Class|AuraAbilitySystemLibrary|GetLiveActorsWithinRadius _returnvalue_2 (Utilities|Array|MakeArray _returnvalue_2) (Variables|Default|GetAttackRadius) _output_get_2))
              (for _array_element _outoverlappingactors
                (if (Class|AuraAbilitySystemLibrary|IsNotFriend (Ability|GetAvatarActorfromActorInfo) _array_element)
                  (Class|AuraDamageGameplayAbility|CauseDamage _array_element)
                  (Variables|Default|SetHasHitTarget true)))
              (if (Variables|Default|GetHasHitTarget)
                (bind _returnvalue_6 (Class|EnemyInterface|GetCombatTarget(Message) (Ability|GetAvatarActorfromActorInfo)))
                (Class|GameplayAbility|ExecuteGameplayCuewithParams "(TagName=\"GameplayCue.MeleeImpact\")" (Ability|GameplayCue|MakeGameplayCueParameters :AggregatedSourceTags (GameplayTags|MakeGameplayTagContainerfromTag (.MontageTag (Utilities|Struct|BreakTaggedMontage (Variables|Default|GetTaggedMontage)))) :Location (Variables|Default|GetCombatSocketLocation) :EffectCauser (Ability|GetAvatarActorfromActorInfo) :SourceObject _returnvalue_6)))
              ;[1 1 1] Should we end the ability here? The animation playing can be interrupted and since, not worked properly
              (Ability|EndAbility))))
        (:OnInterrupted
          (Ability|EndAbility :!label _label))
        (:OnCancelled
          (goto _label))))
    (:Is%20Not%20Valid
      (Development|PrintString "[ERROR]: CombatActor is not valid in GA_MeleeAttack. Cannot warp to CombatTarget" true true "(R=1.000000,G=0.037092,B=0.126759,A=1.000000)")
      (Ability|EndAbility))))

(event Ability|EventOnEndAbility
  (params (bWasCancelled :type Boolean)))