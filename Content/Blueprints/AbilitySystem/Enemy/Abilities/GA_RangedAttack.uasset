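; GA_RangedAttack is an enemy gameplay ability that fires a projectile at the avatar's combat target.
; It turns the avatar toward the target's location captured on activation, then plays a random tagged attack montage.
; When that montage's gameplay event arrives, it spawns the projectile from the montage's socket tag toward the stored location.
; The ability ends right after spawning, or when the montage completes, is interrupted or is cancelled.
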(event Ability|EventActivateAbility
  (bind _returnvalue (Ability|GetAvatarActorfromActorInfo))
  (bind _returnvalue_2 (Class|EnemyInterface|GetCombatTarget(Message) _returnvalue))
  (bind _output_get (Variables|Default|SetTargetLocation (Transformation|GetActorLocation _returnvalue_2)))
  (Class|CombatInterface|SetFacingTarget(Message) _returnvalue _output_get)
  (bind _returnvalue_3 (Class|CombatInterface|GetAttackMontages(Message) _returnvalue))
  (bind _output_get_2 (Variables|Default|SetTaggedAttackAnimation (Class|AuraDamageGameplayAbility|GetRandomTaggedMontagefromArray _returnvalue_3)))
  (|PlayMontageandWaitProxy "None" (.Montage (Utilities|Struct|BreakTaggedMontage _output_get_2)) 1.0 "None" true 1.0 0.0 false
    (:then
      (Ability|Tasks|WaitGameplayEvent (.MontageTag (Utilities|Struct|BreakTaggedMontage _output_get_2)) 0 true
        (:EventReceived
          (Class|CombatInterface|GetCombatSocketLocation(Message) (Ability|GetAvatarActorfromActorInfo) (.SocketTag (Utilities|Struct|BreakTaggedMontage _output_get_2)))
          (Class|AuraProjectileSpell|SpawnProjectile (Variables|Default|GetTargetLocation) (.SocketTag (Utilities|Struct|BreakTaggedMontage _output_get_2)))
          ;[1 1 1] I think we need not to EndAbility right here. The PlayMontageAndWait node is set to EndAbility when the animation ends
          (Ability|EndAbility))))
    (:OnCompleted
      (Ability|EndAbility :!label _label))
    (:OnInterrupted
      (goto _label))
    (:OnCancelled
      (goto _label))))

(event Ability|EventOnEndAbility
  (params (bWasCancelled :type Boolean)))