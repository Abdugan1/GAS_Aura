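; Main menu scene actor that shows the menu UI and animates a floating fireball.
; On BeginPlay it plays menu music, adds the WBP_MainMenu widget and switches the player to UI-only input with a visible cursor.
; Each tick it bobs the fireball vertically around its starting location using a sine of accumulated time scaled by an amplitude, resetting the timer after each full period.
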(event EventBeginPlay
  (bind _returnvalue (Game|GetPlayerController 0))
  (Variables|Default|SetFireBallInitialLocation (Transformation|GetWorldLocation (Variables|Default|GetFireball)))
  (Audio|PlaySound2D "/Game/Assets/Sounds/Music/Music_MainMenu.Music_MainMenu" 1.0 1.0 0.0 0 0)
  (bind _returnvalue_2 (UserInterface|CreateWidget "/Game/Blueprints/UI/MainMenu/WBP_MainMenu.WBP_MainMenu_C"))
  (UserInterface|Viewport|AddtoViewport _returnvalue_2 0)
  (Input|SetInputModeUIOnly _returnvalue _returnvalue_2 "DoNotLock" false)
  (Variables|/Script/Engine.PlayerController|SetbShowMouseCursor _returnvalue true))

(event Collision|EventActorBeginOverlap
  (params (OtherActor :type Actor%20Object%20Reference)))

(event EventTick
  (params (DeltaSeconds :type Float%20%28single-precision%29))
  (CallFunction|UpdateTime DeltaSeconds)
  (Transformation|SetWorldLocation (Variables|Default|GetFireball) (+ (Variables|Default|GetFireBallInitialLocation) (Math|Vector|MakeVector 0.0 0.0 (CallFunction|SineTime))) false false))

(fn ConstructionScript)

(fn UpdateTime
  (params (A :type Float%20%28double-precision%29))
  (bind _output_get (Variables|Default|SetTime (+ A (Variables|Default|GetTime))))
  (if (> _output_get (* (Math|Trig|GetPI) 2.0))
    (Variables|Default|SetTime 0.0)))

(fn SineTime
  (return (* (Math|Trig|Sin(Radians) (Variables|Default|GetTime)) (Variables|Default|GetAplitude))))